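; Turtle2 is a turtle Blueprint that alternates between moving and stopped states.
; BeginPlay runs an endless Delay-driven loop that flips IsMoving and sets Speed between a fixed value and zero, with a longer moving phase than pause.
; Tick and the construction script only call their parents, and nothing in this file applies Speed to movement.
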(event EventBeginPlay
  (if (Variables|Default|GetisMoving) :!label _label
    (Utilities|FlowControl|Delay 1.0)
    (Variables|Default|SetSpeed 0.0)
    (Variables|Default|SetisMoving false)
    (goto _label)
    (else
      (Utilities|FlowControl|Delay 0.5)
      (Variables|Default|SetSpeed 1e+02)
      (Variables|Default|SetisMoving true)
      (goto _label))))

(event EventTick
  (params (DeltaSeconds :type Float%20%28single-precision%29))
  (|CallParentFunction DeltaSeconds))

(fn ConstructionScript
  (|CallParentFunction))