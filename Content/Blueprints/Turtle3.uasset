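; Turtle Blueprint that periodically reverses the sign of its Speed, alternating between forward and backward phases.
; BeginPlay runs an endless Delay loop that flips Speed and IsForward, waiting longer in the forward phase than in the backward one.
; Tick and the construction script only call the parent, and nothing in these graphs applies Speed to movement.
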(event EventBeginPlay
  (if (Variables|Default|GetisForward) :!label _label
    (Utilities|FlowControl|Delay 1.0)
    (Variables|Default|SetSpeed (* -1 (Variables|Default|GetSpeed)))
    (Variables|Default|SetisForward false)
    (goto _label)
    (else
      (Utilities|FlowControl|Delay 0.5)
      (Variables|Default|SetSpeed (* -1 (Variables|Default|GetSpeed)))
      (Variables|Default|SetisForward true)
      (goto _label))))

(event EventTick
  (params (DeltaSeconds :type Float%20%28single-precision%29))
  (|CallParentFunction DeltaSeconds))

(fn ConstructionScript
  (|CallParentFunction))