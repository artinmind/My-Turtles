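; Overlap-triggered button actor that displays a Number on its text render and spawns an actor at a referenced NestVar actor.
; Entering the box collision plays a sound and spawns the configured class, both at that actor's location.
; It also sets the point light to ColorLight and toggles its visibility twice around a short delay, producing a brief flash.
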(event OnComponentBeginOverlap(Boxcollision)
  (params (OverlappedComponent :type Primitive%20Component%20Object%20Reference) (OtherActor :type Actor%20Object%20Reference) (OtherComp :type Primitive%20Component%20Object%20Reference) (OtherBodyIndex :type Integer) (bFromSweep :type Boolean) (SweepResult :type Hit%20Result%20Structure%20%28by%20ref%29))
  (bind _pointlight (Variables|Default|GetPointLight))
  (bind _nestvar (Variables|Default|GetNestVar))
  (bind _returnvalue (Transformation|GetActorLocation _nestvar))
  (Audio|PlaySoundatLocation (Variables|Default|GetSound) _returnvalue "0, 0, 0" 1.0 1.0 0.0 0 0 0)
  (Game|SpawnActorfromClass (Variables|Default|GetClass) (Math|Conversions|ToTransform(Vector) _returnvalue) "Undefined" 0 0)
  (Rendering|Components|Light|SetLightColor _pointlight (Variables|Default|GetColor_light) true)
  (Rendering|ToggleVisibility _pointlight false)
  (Utilities|FlowControl|Delay 0.3)
  (Rendering|ToggleVisibility (Variables|Default|GetPointLight) false))

(event EventBeginPlay
  (Rendering|Components|TextRender|SetText (Variables|Default|GetTextRender) (Variables|Default|GetNumber)))

(fn ConstructionScript)